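; A moving platform Blueprint that the player can pause or slow with the E key, depending on character abilities.
; Overlapping Player_Touch plays a timeline moving the platform from its start to EndPoint, and the character leaving reverses it.
; Tick polls the character's SlowMech and PauseMech flags to enable input.
; E toggles timeline stop/play with PauseMech, or briefly drops the play rate with SlowMech.
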(event `self.ReceiveTick`
  (params (DeltaSeconds :type "Float (single-precision)"))
  (bind _asthird_person_character (cast `/Game/Player/ThirdPersonCharacter` (`GameplayStatics.GetPlayerCharacter` 0)))
  (if (`/Game/Player/ThirdPersonCharacter.SlowMech` _asthird_person_character)
    (set `self.SlowMovement` true)
    (`self.EnableInput` (`GameplayStatics.GetPlayerController` 0) :!label _label)
    (else
      (set `self.SlowMovement` false)
      (if (`/Game/Player/ThirdPersonCharacter.PauseMech` _asthird_person_character)
        (goto _label)))))

(event `self.ReceiveBeginPlay`
  (`self.setLocations`))

(event `self.Player_Touch.OnComponentBeginOverlap`
  (params (OverlappedComponent :type "PrimitiveComponent Object Reference") (OtherActor :type "Actor Object Reference") (OtherComp :type "PrimitiveComponent Object Reference") (OtherBodyIndex :type Integer) (bFromSweep :type Boolean) (SweepResult :type "HitResult Structure (by ref)"))
  (bind (_direction _newtrack_0) (`Timeline|platformMove` :!label _label_2)
    (:`Update`
      (`SceneComponent.K2_SetWorldLocation` (`self.platform`) (`KismetMathLibrary.VLerp` (`self.startLocation`) (`self.endLocation`) _newtrack_0) false false))))

(event `Key|E`
  (params (Key :type "Key Structure"))
  (:`Pressed`
    (if (`/Game/Player/ThirdPersonCharacter.PauseMech` (stale `self.ReceiveTick` _asthird_person_character))
      (`/Engine/EditorBlueprintResources/StandardMacros.FlipFlop`
        (:`A`
          (goto _label_2 :!via `Stop`))
        (:`B`
          (goto _label_2))))))

(event `self.Player_Touch.OnComponentEndOverlap`
  (params (OverlappedComponent :type "PrimitiveComponent Object Reference") (OtherActor :type "Actor Object Reference") (OtherComp :type "PrimitiveComponent Object Reference") (OtherBodyIndex :type Integer))
  (cast `/Game/Player/ThirdPersonCharacter` OtherActor)
  (`self.DisableInput` null)
  (goto _label_2 :!via `Reverse`))

(event `Key|E`
  (params (Key :type "Key Structure"))
  (:`Pressed`
    (if (`self.SlowMovement`)
      (`TimelineComponent.SetPlayRate` (`self.platformMove`) 0.25)
      (`KismetSystemLibrary.Delay` 0.5)
      (`TimelineComponent.SetPlayRate` (`self.platformMove`) 1.0))))

(fn `setLocations`
  (set `self.startLocation` (`SceneComponent.K2_GetComponentLocation` (`self.platform`)))
  (set `self.endLocation` (`SceneComponent.K2_GetComponentLocation` (`self.End_Point`)))
  (`TimelineComponent.SetPlayRate` (`self.platformMove`) (`self.playRate`)))

(fn `UserConstructionScript`)