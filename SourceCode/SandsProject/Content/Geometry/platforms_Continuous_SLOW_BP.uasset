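; Continuously moving platform that the player can click to slow down temporarily.
; On BeginPlay it records platform and end point locations, enables mouse click events, and runs a timeline that lerps the platform between them.
; Clicking it while the ThirdPersonCharacter's SlowMech is set cuts the timeline rate for ten seconds, then restores it to 1.0 rather than the configured PlayRate.
; The Player_Touch overlap only casts and has no effect.
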(event `self.ReceiveBeginPlay`
  (bind _returnvalue (`GameplayStatics.GetPlayerController` 0))
  (`self.setLocations`)
  (set `PlayerController.bEnableMouseOverEvents` true _returnvalue)
  (set `PlayerController.bEnableClickEvents` true _returnvalue)
  (bind (_direction _continuousmovement) (`Timeline|platformMove`)
    (:`Update`
      (`SceneComponent.K2_SetWorldLocation` (`self.platform`) (`KismetMathLibrary.VLerp` (`self.startLocation`) (`self.endLocation`) _continuousmovement) false false))))

(event `self.Player_Touch.OnComponentBeginOverlap`
  (params (OverlappedComponent :type "PrimitiveComponent Object Reference") (OtherActor :type "Actor Object Reference") (OtherComp :type "PrimitiveComponent Object Reference") (OtherBodyIndex :type Integer) (bFromSweep :type Boolean) (SweepResult :type "HitResult Structure (by ref)"))
  (cast `/Game/Player/ThirdPersonCharacter` OtherActor))

(event `self.ReceiveActorOnClicked`
  (params (ButtonPressed :type "Key Structure"))
  (bind _platformmove (`self.platformMove`))
  (bind _asthird_person_character (cast `/Game/Player/ThirdPersonCharacter` (`GameplayStatics.GetPlayerPawn` 0)))
  (if (`/Game/Player/ThirdPersonCharacter.SlowMech` _asthird_person_character)
    (`TimelineComponent.SetPlayRate` _platformmove 0.25)
    (`KismetSystemLibrary.Delay` 10.0)
    (`TimelineComponent.SetPlayRate` _platformmove 1.0)))

(fn `setLocations`
  (set `self.startLocation` (`SceneComponent.K2_GetComponentLocation` (`self.platform`)))
  (set `self.endLocation` (`SceneComponent.K2_GetComponentLocation` (`self.End_Point`)))
  (`TimelineComponent.SetPlayRate` (`self.platformMove`) (`self.playRate`)))

(fn `UserConstructionScript`)