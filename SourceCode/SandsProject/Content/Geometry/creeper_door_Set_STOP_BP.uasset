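; A creeper door set whose left and right doors swing with the player's position and can be frozen by clicking.
; Every tick the two doors take opposite yaw rotations from the character's world Y location scaled by Swing.
; When PauseMech is set on the character, a click calls its MechanicCheck and halts the doors' rotation for ten seconds.
; BeginPlay enables mouse-over and click events on the player controller.
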(event `self.ReceiveBeginPlay`
  (bind _returnvalue (`GameplayStatics.GetPlayerController` 0))
  (set `PlayerController.bEnableMouseOverEvents` true _returnvalue)
  (set `PlayerController.bEnableClickEvents` true _returnvalue))

(event `self.ReceiveTick`
  (params (DeltaSeconds :type "Float (single-precision)"))
  (bind _asthird_person_character (cast `/Game/Player/ThirdPersonCharacter` (`GameplayStatics.GetPlayerCharacter` 0)))
  (if (not (`self.clicked`))
    (bind (_returnvalue_x _returnvalue_y) (`KismetMathLibrary.BreakVector` (`self.K2_GetActorLocation` _asthird_person_character)))
    (bind _returnvalue (* _returnvalue_y (`self.swing`)))
    (`SceneComponent.K2_SetWorldRotation` (`self.LeftDoor`) (`KismetMathLibrary.MakeRotator` 0.0 0.0 (* _returnvalue -1.0)) false false)
    (`SceneComponent.K2_SetWorldRotation` (`self.RightDoor`) (`KismetMathLibrary.MakeRotator` 0.0 0.0 _returnvalue) false false)))

(event `self.ReceiveActorOnClicked`
  (params (ButtonPressed :type "Key Structure"))
  (bind _asthird_person_character (cast `/Game/Player/ThirdPersonCharacter` (`GameplayStatics.GetPlayerPawn` 0)))
  (if (`/Game/Player/ThirdPersonCharacter.PauseMech` _asthird_person_character)
    (bind _asthird_person_character_2 (cast `/Game/Player/ThirdPersonCharacter` (`GameplayStatics.GetPlayerCharacter` 0)))
    (`/Game/Player/ThirdPersonCharacter.MechanicCheck` _asthird_person_character_2)
    (set `self.clicked` true)
    (`KismetSystemLibrary.Delay` 10.0)
    (set `self.clicked` false)))

(fn `UserConstructionScript`)