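; Pillar actor that starts toppling at BeginPlay, which the player can freeze with a mouse click.
; The FallDown timeline drives the mesh's relative X rotation at a configurable play rate.
; Tick detects a fresh left click while hovered; if the character's PauseMech is set, it stops the timeline, calls MechanicCheck and resumes after a delay.
; The stored start and fall locations are unused here, and the PlayerTouch overlap only casts.
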(event `self.ReceiveBeginPlay`
  (bind _returnvalue (`GameplayStatics.GetPlayerController` 0))
  (`self.setLocations`)
  (set `PlayerController.bEnableMouseOverEvents` true _returnvalue)
  (set `PlayerController.bEnableClickEvents` true _returnvalue)
  (bind (_direction _timefloat) (`Timeline|fallDown` :!label _label)
    (:`Update`
      (`SceneComponent.K2_SetRelativeRotation` (`self.StaticMeshComponent`) (`KismetMathLibrary.MakeRotator` (.x (`KismetMathLibrary.MakeVector` _timefloat))) false false))))

(event `self.ReceiveActorBeginCursorOver`
  (set `self.Hover` true))

(event `self.PlayerTouch.OnComponentBeginOverlap`
  (params (OverlappedComponent :type "PrimitiveComponent Object Reference") (OtherActor :type "Actor Object Reference") (OtherComp :type "PrimitiveComponent Object Reference") (OtherBodyIndex :type Integer) (bFromSweep :type Boolean) (SweepResult :type "HitResult Structure (by ref)"))
  (cast `/Game/Player/ThirdPersonCharacter` OtherActor))

(event `self.ReceiveActorEndCursorOver`
  (set `self.Hover` false))

(event `self.ReceiveTick`
  (params (DeltaSeconds :type "Float (single-precision)"))
  (if (`PlayerController.IsInputKeyDown` (`GameplayStatics.GetPlayerController` 0) "LeftMouseButton")
    (if (not (`self.Click`))
      (set `self.Click` true)
      (if (`self.Hover`)
        (bind _asthird_person_character (cast `/Game/Player/ThirdPersonCharacter` (`GameplayStatics.GetPlayerPawn` 0)))
        (if (`/Game/Player/ThirdPersonCharacter.PauseMech` _asthird_person_character)
          (`|ExecutionSequence`
            (:`then_0`
              (goto _label :!via `Stop`))
            (:`then_1`
              (bind _asthird_person_character_2 (cast `/Game/Player/ThirdPersonCharacter` (`GameplayStatics.GetPlayerCharacter` 0)))
              (`/Game/Player/ThirdPersonCharacter.MechanicCheck` _asthird_person_character_2)
              (`KismetSystemLibrary.Delay` 20.0)
              (goto _label))))))
    (else
      (set `self.Click` false))))

(fn `setLocations`
  (set `self.StartLocation` (`SceneComponent.K2_GetComponentLocation` (`self.StaticMeshComponent`)))
  (set `self.FallLocation` (`SceneComponent.K2_GetComponentLocation` (`self.FallPoint`)))
  (`TimelineComponent.SetPlayRate` (`self.fallDown`) (`self.playRate`)))

(fn `UserConstructionScript`)