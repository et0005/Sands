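; A creeper door set: a pair of doors that swing in response to the player's position along the world Y axis.
; Every Tick it casts the player character to ThirdPersonCharacter and multiplies its Y location by Swing to get a yaw.
; LeftDoor takes that yaw as world rotation and RightDoor takes its negation, with no clamping, interpolation or trigger volume.
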(event `self.ReceiveTick`
  (params (DeltaSeconds :type "Float (single-precision)"))
  (bind _asthird_person_character (cast `/Game/Player/ThirdPersonCharacter` (`GameplayStatics.GetPlayerCharacter` 0)))
  (bind (_returnvalue_x _returnvalue_y) (`KismetMathLibrary.BreakVector` (`self.K2_GetActorLocation` _asthird_person_character)))
  (bind _returnvalue (* _returnvalue_y (`self.swing`)))
  (`SceneComponent.K2_SetWorldRotation` (`self.LeftDoor`) (`KismetMathLibrary.MakeRotator` 0.0 0.0 _returnvalue) false false)
  (`SceneComponent.K2_SetWorldRotation` (`self.RightDoor`) (`KismetMathLibrary.MakeRotator` 0.0 0.0 (* _returnvalue -1.0)) false false))

(fn `UserConstructionScript`)