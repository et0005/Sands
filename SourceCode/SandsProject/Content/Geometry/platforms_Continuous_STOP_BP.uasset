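; A moving platform actor that the player can click to temporarily freeze.
; On BeginPlay it caches start and end component positions and plays the PlatformMove timeline at a set rate to lerp between them.
; With mouse events enabled, a click while the character's PauseMech is set stops the timeline, calls MechanicCheck, then resumes after a delay.
; The touch overlap handler only casts to the character and does nothing further.
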(event `self.ReceiveBeginPlay`
  (bind _returnvalue (`GameplayStatics.GetPlayerController` 0))
  (`self.setLocations`)
  (set `PlayerController.bEnableMouseOverEvents` true _returnvalue)
  (set `PlayerController.bEnableClickEvents` true _returnvalue)
  (bind (_direction _newtrack_0) (`Timeline|platformMove` :!label _label)
    (:`Update`
      (`SceneComponent.K2_SetWorldLocation` (`self.platform`) (`KismetMathLibrary.VLerp` (`self.startLocation`) (`self.endLocation`) _newtrack_0) false false))))

(event `self.Player_Touch.OnComponentBeginOverlap`
  (params (OverlappedComponent :type "PrimitiveComponent Object Reference") (OtherActor :type "Actor Object Reference") (OtherComp :type "PrimitiveComponent Object Reference") (OtherBodyIndex :type Integer) (bFromSweep :type Boolean) (SweepResult :type "HitResult Structure (by ref)"))
  (cast `/Game/Player/ThirdPersonCharacter` OtherActor))

(event `self.ReceiveActorOnClicked`
  (params (ButtonPressed :type "Key Structure"))
  (bind _asthird_person_character (cast `/Game/Player/ThirdPersonCharacter` (`GameplayStatics.GetPlayerPawn` 0)))
  (if (`/Game/Player/ThirdPersonCharacter.PauseMech` _asthird_person_character)
    (`|ExecutionSequence`
      (:`then_0`
        (goto _label :!via `Stop`))
      (:`then_1`
        (bind _asthird_person_character_2 (cast `/Game/Player/ThirdPersonCharacter` (`GameplayStatics.GetPlayerCharacter` 0)))
        (`/Game/Player/ThirdPersonCharacter.MechanicCheck` _asthird_person_character_2)
        (`KismetSystemLibrary.Delay` 20.0)
        (goto _label)))))

(fn `setLocations`
  (set `self.startLocation` (`SceneComponent.K2_GetComponentLocation` (`self.platform`)))
  (set `self.endLocation` (`SceneComponent.K2_GetComponentLocation` (`self.End_Point`)))
  (`TimelineComponent.SetPlayRate` (`self.platformMove`) (`self.playRate`)))

(fn `UserConstructionScript`)