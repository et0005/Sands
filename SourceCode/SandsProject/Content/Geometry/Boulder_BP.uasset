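; Boulder trap that falls when the player enters its trigger and sends a player who touches its sphere collider back to their start location.
; A FallDown timeline lerps the mesh between positions cached at BeginPlay.
; With SlowMech active, clicking the hovered boulder, detected by Tick polling, calls MechanicCheck and temporarily slows the fall before setting normal speed.
; Roll and ReverseFall timelines are unconnected and never run.
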(event `self.PlayerTouch.OnComponentBeginOverlap`
  (params (OverlappedComponent :type "PrimitiveComponent Object Reference") (OtherActor :type "Actor Object Reference") (OtherComp :type "PrimitiveComponent Object Reference") (OtherBodyIndex :type Integer) (bFromSweep :type Boolean) (SweepResult :type "HitResult Structure (by ref)"))
  (cast `/Game/Player/ThirdPersonCharacter` OtherActor)
  (bind (_direction _timefloat) (`Timeline|fallDown`)
    (:`Update`
      (`SceneComponent.K2_SetWorldLocation` (`self.StaticMeshComponent`) (`KismetMathLibrary.VLerp` (`self.startLocation`) (`self.FallLocation`) _timefloat) false false))))

(event `self.ReceiveActorBeginCursorOver`
  (set `self.Hover` true))

(event `self.ReceiveActorEndCursorOver`
  (set `self.Hover` false))

(event `self.ReceiveTick`
  (params (DeltaSeconds :type "Float (single-precision)"))
  (bind _falldown (`self.fallDown`))
  (if (`PlayerController.IsInputKeyDown` (`GameplayStatics.GetPlayerController` 0) "LeftMouseButton")
    (if (not (`self.Click`))
      (set `self.Click` true)
      (if (`self.Hover`)
        (bind _asthird_person_character (cast `/Game/Player/ThirdPersonCharacter` (`GameplayStatics.GetPlayerPawn` 0)))
        (if (`/Game/Player/ThirdPersonCharacter.SlowMech` _asthird_person_character)
          (bind _asthird_person_character_2 (cast `/Game/Player/ThirdPersonCharacter` (`GameplayStatics.GetPlayerCharacter` 0)))
          (`/Game/Player/ThirdPersonCharacter.MechanicCheck` _asthird_person_character_2)
          (`TimelineComponent.SetPlayRate` _falldown 0.25)
          (`KismetSystemLibrary.Delay` 10.0)
          (`TimelineComponent.SetPlayRate` _falldown 1.0))))
    (else
      (set `self.Click` false))))

(event `self.ReceiveBeginPlay`
  (bind _returnvalue (`GameplayStatics.GetPlayerController` 0))
  (`self.setLocations`)
  (set `PlayerController.bEnableMouseOverEvents` true _returnvalue)
  (set `PlayerController.bEnableClickEvents` true _returnvalue))

(event `self.sphereCollider.OnComponentBeginOverlap`
  (params (OverlappedComponent :type "PrimitiveComponent Object Reference") (OtherActor :type "Actor Object Reference") (OtherComp :type "PrimitiveComponent Object Reference") (OtherBodyIndex :type Integer) (bFromSweep :type Boolean) (SweepResult :type "HitResult Structure (by ref)"))
  (bind _asthird_person_character (cast `/Game/Player/ThirdPersonCharacter` OtherActor))
  (`self.K2_SetActorLocation` _asthird_person_character (`/Game/Player/ThirdPersonCharacter.startLocation` _asthird_person_character) false false))

(fn `setLocations`
  (set `self.StartLocation` (`SceneComponent.K2_GetComponentLocation` (`self.StaticMeshComponent`)))
  (set `self.FallLocation` (`SceneComponent.K2_GetComponentLocation` (`self.FallPoint`)))
  (set `self.EndLocation` (`SceneComponent.K2_GetComponentLocation` (`self.EndPoint`)))
  (`TimelineComponent.SetPlayRate` (`self.fallDown`) (`self.playRate`)))

(fn `UserConstructionScript`)