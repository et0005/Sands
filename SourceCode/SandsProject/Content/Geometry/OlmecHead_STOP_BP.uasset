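; Olmec head platform that falls and rolls when the third-person character overlaps its trigger, and can be paused by a mouse click.
; The PlatformMove timeline lerps it from its start to the EndPoint and drives its roll, at a play rate set on BeginPlay.
; If the character's PauseMech is true, a click stops the timeline, calls MechanicCheck on the character and resumes movement after a long delay.
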(event `self.ReceiveBeginPlay`
  (bind _returnvalue (`GameplayStatics.GetPlayerController` 0))
  (`self.setLocations`)
  (set `PlayerController.bEnableMouseOverEvents` true _returnvalue)
  (set `PlayerController.bEnableClickEvents` true _returnvalue))

(event `self.Player_Touch.OnComponentBeginOverlap`
  (params (OverlappedComponent :type "PrimitiveComponent Object Reference") (OtherActor :type "Actor Object Reference") (OtherComp :type "PrimitiveComponent Object Reference") (OtherBodyIndex :type Integer) (bFromSweep :type Boolean) (SweepResult :type "HitResult Structure (by ref)"))
  (cast `/Game/Player/ThirdPersonCharacter` OtherActor)
  (bind (_direction _falling _rolling _vertical_movement_2_0) (`Timeline|platformMove` :!label _label)
    (:`Update`
      (`|ExecutionSequence`
        (:`then_0`
          (`SceneComponent.K2_SetWorldLocation` (`self.platform`) (`KismetMathLibrary.VLerp` (`self.startLocation`) (`self.endLocation`) _falling) false false))
        (:`then_1`
          (`SceneComponent.K2_SetRelativeRotation` (`self.platform`) (`KismetMathLibrary.MakeRotator` (.x (`KismetMathLibrary.MakeVector` _rolling)) 0.0 90.0) false false))
        (:`then_2`
          (`KismetSystemLibrary.Delay` 1.2))))
    (:`Finished`
      (`SceneComponent.K2_SetWorldLocation` (`self.platform`) (`KismetMathLibrary.VLerp` (`KismetMathLibrary.MakeVector` (.x (`SceneComponent.K2_GetComponentLocation` (`self.platform`))) (.y (`SceneComponent.K2_GetComponentLocation` (`self.platform`))) _vertical_movement_2_0) (`self.endLocation`) _vertical_movement_2_0) false false))))

(event `self.ReceiveActorOnClicked`
  (params (ButtonPressed :type "Key Structure"))
  (bind _asthird_person_character (cast `/Game/Player/ThirdPersonCharacter` (`GameplayStatics.GetPlayerPawn` 0)))
  (if (`/Game/Player/ThirdPersonCharacter.PauseMech` _asthird_person_character)
    (`|ExecutionSequence`
      (:`then_0`
        (goto _label :!via `Stop`))
      (:`then_1`
        (bind _asthird_person_character_2 (cast `/Game/Player/ThirdPersonCharacter` (`GameplayStatics.GetPlayerCharacter` 0)))
        (`/Game/Player/ThirdPersonCharacter.MechanicCheck` _asthird_person_character_2)
        (`KismetSystemLibrary.Delay` 20.0)
        (goto _label)))))

(fn `setLocations`
  (set `self.startLocation` (`SceneComponent.K2_GetComponentLocation` (`self.platform`)))
  (set `self.endLocation` (`SceneComponent.K2_GetComponentLocation` (`self.End_Point`)))
  (`TimelineComponent.SetPlayRate` (`self.platformMove`) (`self.playRate`)))

(fn `UserConstructionScript`)