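; Vertical moving platform that travels toward an end point while the third-person character overlaps its touch volume and reverses when the character leaves.
; A timeline lerps the platform between start and EndPoint locations cached at BeginPlay, at a configurable play rate.
; Input is enabled only during overlap, so holding left mouse stops the platform and releasing resumes forward travel.
; A flip-flop pause function is defined but never called here.
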(event `self.ReceiveBeginPlay`
  (`self.setLocations`))

(event `self.Player_Touch.OnComponentBeginOverlap`
  (params (OverlappedComponent :type "PrimitiveComponent Object Reference") (OtherActor :type "Actor Object Reference") (OtherComp :type "PrimitiveComponent Object Reference") (OtherBodyIndex :type Integer) (bFromSweep :type Boolean) (SweepResult :type "HitResult Structure (by ref)"))
  (cast `/Game/Player/ThirdPersonCharacter` OtherActor)
  (`self.EnableInput` (`GameplayStatics.GetPlayerController` 0))
  (bind (_direction _newtrack_0) (`Timeline|platformMove` :!label _label)
    (:`Update`
      (`SceneComponent.K2_SetWorldLocation` (`self.platform`) (`KismetMathLibrary.VLerp` (`self.startLocation`) (`self.endLocation`) _newtrack_0) false false))))

(event `Key|LeftMouseButton`
  (params (Key :type "Key Structure"))
  (:`Pressed`
    (goto _label :!via `Stop`))
  (:`Released`
    (goto _label)))

(event `self.Player_Touch.OnComponentEndOverlap`
  (params (OverlappedComponent :type "PrimitiveComponent Object Reference") (OtherActor :type "Actor Object Reference") (OtherComp :type "PrimitiveComponent Object Reference") (OtherBodyIndex :type Integer))
  (cast `/Game/Player/ThirdPersonCharacter` OtherActor)
  (`self.DisableInput` null)
  (goto _label :!via `Reverse`))

(fn `PauseMovementLogic`
  (`/Engine/EditorBlueprintResources/StandardMacros.FlipFlop`
    (:`A`
      (set `self.PauseMovement` true))
    (:`B`
      (set `self.PauseMovement` false))))

(fn `setLocations`
  (set `self.startLocation` (`SceneComponent.K2_GetComponentLocation` (`self.platform`)))
  (set `self.endLocation` (`SceneComponent.K2_GetComponentLocation` (`self.End_Point`)))
  (`TimelineComponent.SetPlayRate` (`self.platformMove`) (`self.playRate`)))

(fn `UserConstructionScript`)