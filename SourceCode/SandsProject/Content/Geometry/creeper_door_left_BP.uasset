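; A creeper door (left side) actor that swings continuously based on the player's position and can be frozen by clicking.
; Each Tick sets its yaw from the negated Y location of the ThirdPersonCharacter scaled by Swing.
; On click, if the character's PauseMech flag is set, it calls MechanicCheck and zeroes Swing, then restores it after a ten-second Delay.
; BeginPlay enables mouse click and hover events on the player controller.
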(event `self.ReceiveBeginPlay`
  (bind _returnvalue (`GameplayStatics.GetPlayerController` 0))
  (set `PlayerController.bEnableMouseOverEvents` true _returnvalue)
  (set `PlayerController.bEnableClickEvents` true _returnvalue))

(event `self.ReceiveTick`
  (params (DeltaSeconds :type "Float (single-precision)"))
  (bind _asthird_person_character (cast `/Game/Player/ThirdPersonCharacter` (`GameplayStatics.GetPlayerCharacter` 0)))
  (bind (_returnvalue_x _returnvalue_y) (`KismetMathLibrary.BreakVector` (`self.K2_GetActorLocation` _asthird_person_character)))
  (`self.K2_SetActorRotation` (`KismetMathLibrary.MakeRotator` 0.0 0.0 (* (* _returnvalue_y -1.0) (`self.swing`)))))

(event `self.ReceiveActorOnClicked`
  (params (ButtonPressed :type "Key Structure"))
  (bind _asthird_person_character (cast `/Game/Player/ThirdPersonCharacter` (`GameplayStatics.GetPlayerPawn` 0)))
  (if (`/Game/Player/ThirdPersonCharacter.PauseMech` _asthird_person_character)
    (bind _asthird_person_character_2 (cast `/Game/Player/ThirdPersonCharacter` (`GameplayStatics.GetPlayerCharacter` 0)))
    (`/Game/Player/ThirdPersonCharacter.MechanicCheck` _asthird_person_character_2)
    (set `self.swing` 0.0)
    (`KismetSystemLibrary.Delay` 10.0)
    (set `self.Swing` 0.06274)))

(fn `UserConstructionScript`)